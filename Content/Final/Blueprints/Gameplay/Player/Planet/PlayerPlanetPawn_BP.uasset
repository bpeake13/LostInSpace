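; PlayerPlanetPawn_BP is the player pawn for planet gameplay, with an arrow that points toward its current destination.
; A SetDestination event stores the target, whose world location Tick uses to rotate the arrow with a look-at rotation from the pawn's location.
; The arrow is hidden when no destination is set and shown otherwise.
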(event `self.ReceiveBeginPlay`)

(event `self.ReceiveActorBeginOverlap`
  (params (OtherActor :type "Actor Object Reference")))

(event `self.ReceiveTick`
  (params (DeltaSeconds :type "Float (single-precision)"))
  (bind _arrow (`self.Arrow`))
  (if (== (`self.Destination`) null)
    (`SceneComponent.SetVisibility` _arrow false false)
    (else
      (`SceneComponent.K2_SetWorldRotation` _arrow (`KismetMathLibrary.FindLookAtRotation` (`self.K2_GetActorLocation`) (`SceneComponent.K2_GetComponentLocation` (`self.Destination`))) false)
      (`SceneComponent.SetVisibility` (`self.Arrow`) true false))))

(event `self.SetDestination`
  (params (newDestination :type "DestinationPoint Object Reference"))
  (set `self.Destination` newDestination))

(fn `UserConstructionScript`)